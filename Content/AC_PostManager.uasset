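; AC_PostManager is a component that captures screenshots and uploads them to a web server over HTTP POST.
; ScreenshotPost saves a padded screenshot under the user's Pictures path, builds multipart form data from it and returns the file as a Texture2D.
; JsonPost sends that body as binary content through VaRest to the base URL plus an endpoint suffix, with no response handling.
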(event EventBeginPlay)

(event EventTick
  (params (DeltaSeconds :type Float%20%28single-precision%29)))

(fn JsonPost
  (params (type :type String) (Boundary :type String) (Content :type Array%20of%20Bytes))
  (bind _returnvalue (Class|VaRestSubsystem|ConstructVaRestRequestExt (|VaRestSubsystem) "POST" "binary"))
  (bind _output_get (LocalVariables|SetJson _returnvalue))
  (Class|VaRestRequestJSON|SetURL _output_get (Utilities|String|Append (LocalVariables|GetUrl) type))
  (Class|VaRestRequestJSON|SetHeader (LocalVariables|GetJson) "Content-Type" (Utilities|String|Append (LocalVariables|GetMultipart) Boundary))
  (Class|VaRestRequestJSON|SetBinaryRequestContent (LocalVariables|GetJson) Content)
  (Class|VaRestRequestJSON|ExecuteProcessRequest (LocalVariables|GetJson)))

(fn ScreenshotPost
  (params (ScreenshotName :type String) (FolderName :type String) (FieldName :type String) (type :type String) (TopPadding :type Float%20%28single-precision%29) (BottomPadding :type Float%20%28single-precision%29) (LeftPadding :type Float%20%28single-precision%29) (RightPadding :type Float%20%28single-precision%29))
  (bind _returnvalue (Class|BLibraryBP|TakeScreenshot ScreenshotName (Utilities|String|Append (Class|BLibraryBP|GetMyPicturesPath) "/" FolderName "/") TopPadding BottomPadding LeftPadding RightPadding))
  (bind (_outboundary _outrequestbody) (Class|BLibraryBP|GenerateMultipartFormData _returnvalue FieldName))
  (CallFunction|JsonPost type _outboundary _outrequestbody)
  (bind _returnvalue_2 (Class|KismetRenderingLibrary|ImportFileasTexture2D _returnvalue))
  (return _returnvalue_2))